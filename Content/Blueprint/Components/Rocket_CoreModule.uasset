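; Core module component of a Rocket that tracks its engine and fuel modules and provides flight control.
; On BeginPlay it caches the owning Rocket and scans its attach parent's direct children for modules; new ones can also register individually.
; Engines refresh their fuel tank links as modules are found or registered.
; Throttle is forwarded to every engine, while roll, pitch and a weakened yaw apply local-axis torque to the Rocket's collision body.
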(event Custom|Yaw
  (params (Amount :type Float%20%28single-precision%29))
  (Class|PrimitiveComponent|AddTorqueinRadians (Variables|/Script/GameBehaviour.Spacecraft|GetCollision (Variables|Default|GetOwner)) (Math|Transform|TransformDirection (Transformation|GetWorldTransform (Variables|/Script/GameBehaviour.Spacecraft|GetCollision (Variables|Default|GetOwner))) (Math|Vector|MakeVector 0.0 0.0 (/ Amount 4.0))) "None" false))

(event Custom|Roll
  (params (Amount :type Float%20%28single-precision%29))
  (Class|PrimitiveComponent|AddTorqueinRadians (Variables|/Script/GameBehaviour.Spacecraft|GetCollision (Variables|Default|GetOwner)) (Math|Transform|TransformDirection (Transformation|GetWorldTransform (Variables|/Script/GameBehaviour.Spacecraft|GetCollision (Variables|Default|GetOwner))) (Math|Vector|MakeVector Amount 0.0 0.0)) "None" false))

(event Custom|Refresh%20Modules
  (Utilities|Array|Clear (Variables|Default|GetEngines))
  (Utilities|Array|Clear (Variables|Default|GetFuel%20Tanks))
  (for _array_element (Components|GetChildrenComponents (Transformation|GetAttachParent) false)
    (Utilities|FlowControl|Sequence
      (:then_0
        (bind _asrocket_engine_module (Utilities|Casting|CastToRocket_EngineModule _array_element))
        (Utilities|Array|Add (Variables|Default|GetEngines) _asrocket_engine_module)
        (Default|RefreshFuelTanks _asrocket_engine_module))
      (:then_1
        (bind _asrocket_fuel_module (Utilities|Casting|CastToRocket_FuelModule _array_element))
        (Utilities|Array|Add (Variables|Default|GetFuel%20Tanks) _asrocket_fuel_module)))))

(event Custom|Pitch
  (params (Amount :type Float%20%28single-precision%29))
  (Class|PrimitiveComponent|AddTorqueinRadians (Variables|/Script/GameBehaviour.Spacecraft|GetCollision (Variables|Default|GetOwner)) (Math|Transform|TransformDirection (Transformation|GetWorldTransform (Variables|/Script/GameBehaviour.Spacecraft|GetCollision (Variables|Default|GetOwner))) (Math|Vector|MakeVector 0.0 Amount 0.0)) "None" false))

(event Custom|Throttle
  (params (Value :type Float%20%28single-precision%29))
  (for _array_element (Variables|Default|GetEngines)
    (Variables|/Game/Blueprint/Components/Rocket_EngineModule.Rocket_EngineModule_C|SetThrottle _array_element Value)))

(event Custom|Register%20Fuel%20Tank
  (params (Fuel%20Tank :type Rocket%20Fuel%20Module%20Object%20Reference))
  (Utilities|Array|AddUnique (Variables|Default|GetFuel%20Tanks) Fuel%20Tank)
  (for _array_element (Variables|Default|GetEngines)
    (Default|RefreshFuelTanks _array_element)))

(event Custom|Register%20Engine
  (params (Engine :type Rocket%20Engine%20Module%20Object%20Reference))
  (Utilities|Array|AddUnique (Variables|Default|GetEngines) Engine)
  (Default|RefreshFuelTanks Engine))

(event EventBeginPlay
  (bind _asrocket (Utilities|Casting|CastToRocket (Components|GetOwner)))
  (Variables|Default|SetOwner _asrocket)
  (CallFunction|RefreshModules))