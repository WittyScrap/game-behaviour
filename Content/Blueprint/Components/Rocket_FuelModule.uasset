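; Rocket fuel module component that stores a fuel amount and exposes it for reading and consumption.
; DrawFuel subtracts the requested amount and clamps the remainder at zero, without reporting any shortfall.
; GetMass extends the parent's mass with the remaining fuel scaled by a fixed factor, so the module gets lighter as fuel drains.
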(event EventBeginPlay)

(event EventTick
  (params (DeltaSeconds :type Float%20%28single-precision%29)))

(fn GetFuel
  (return (Variables|Default|GetFuel)))

(fn DrawFuel
  (params (Amount :type Float%20%28single-precision%29))
  (Variables|Default|SetFuel (Math|Float|Max(Float) (- (Variables|Default|GetFuel) Amount) 0.0)))

(fn GetMass
  (return (+ (|CallParentFunction) (* (Variables|Default|GetFuel) 1e+03))))