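; Rocket engine module component for a Spacecraft owner that applies force to it each tick while fuel remains.
; RefreshFuelTanks collects sibling Rocket_FuelModule components under the attach parent, whose fuel is summed to gate thrust.
; Fuel draw splits across tanks by throttle, but Tick passes zero delta time, so none drains.
; GetForce's up-vector, Power and Throttle calculation is left unconnected.
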(event Custom|Refresh%20Fuel%20Tanks
  (Utilities|Array|Clear (Variables|Default|GetFuel%20Tanks))
  (for _array_element (Components|GetChildrenComponents (Transformation|GetAttachParent) false)
    (bind _asrocket_fuel_module (Utilities|Casting|CastToRocket_FuelModule _array_element))
    (Utilities|Array|Add (Variables|Default|GetFuel%20Tanks) _asrocket_fuel_module)))

(event EventBeginPlay
  (bind _asspacecraft (Utilities|Casting|CastToSpacecraft (Components|GetOwner))
    (:then
      (Variables|Default|SetOwner _asspacecraft))
    (:CastFailed
      (Development|PrintString "Error: Rocket modules must be attached to a rocket actor" true true "(R=1.000000,G=0.061242,B=0.000000,A=1.000000)"))))

(event EventTick
  (params (DeltaSeconds :type Float%20%28single-precision%29))
  (bind _fuel (CallFunction|GetFuelAmount))
  (if (> _fuel 0.0)
    (CallFunction|DrawFuelAll 0.0)
    (Class|Spacecraft|AddForce (Variables|Default|GetOwner) (Utilities|GetForce))))

(fn GetFuelAmount
  (for _array_element (Variables|Default|GetFuel%20Tanks)
    (LocalVariables|SetTotal%20Fuel (+ (Variables|/Game/Blueprint/Components/Rocket_FuelModule.Rocket_FuelModule_C|GetFuel _array_element) (LocalVariables|GetTotal%20Fuel))))
  (return (LocalVariables|GetTotal%20Fuel)))

(fn DrawFuelAll
  (params (Delta%20Seconds :type Float%20%28single-precision%29))
  (for _array_element (Variables|Default|GetFuel%20Tanks)
    (Default|DrawFuel _array_element (* Delta%20Seconds (/ (Variables|Default|GetFuel%20Drain%20/%20Second) (Math|Conversions|ToFloat(Integer) (Utilities|Array|Length (Variables|Default|GetFuel%20Tanks)))) (Variables|Default|GetThrottle)))))