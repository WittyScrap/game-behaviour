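; Player pawn that runs a solar system sim, spawning configured planets, orbiting them around the first, and managing rockets and the system UI.
; Focus requests from UI or keys glide a zoomable, pannable gimbal camera to a body, optionally aligning its up axis to a rocket's parent body.
; A focused rocket takes throttle, torque and launch input, while the directional light is re-aimed each tick from the system origin toward the camera pivot.
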(event Custom|Focus
  (params (Planet :type Actor%20Object%20Reference))
  ;[1 1 1] Set focus point
  (Utilities|IsValid Planet
    (:Is%20Valid
      (bind _output_get (Variables|Default|SetFocus%20Target Planet))
      (Utilities|CraftFocus _output_get
        (:Success
          _)
        (:Fail
          (Variables|Default|SetCamera%20Pan%20Up%20Axis (Transformation|GetActorUpVector))))
      (Variables|Default|SetCamera%20Pan%20Amount 0.0)
      (Development|PrintString (Utilities|String|Append "Focusing on " (Utilities|GetDisplayName _output_get)))
      (bind _value (Timeline|Focus_Transition PlayFromStart)))))

(event Custom|Generate%20UI
  ;[1 1 1] UI generation
  (Viewport|RemoveAllWidgets)
  (bind _returnvalue (UserInterface|CreateWidget "/Game/Blueprint/UI/SolarSystemUI.SolarSystemUI_C" (Game|GetPlayerController 0)))
  (bind _output_get (Variables|Default|SetUI _returnvalue))
  (UserInterface|Viewport|AddtoViewport _output_get 0)
  (for _array_element (Variables|Default|GetPlanets)
    (Default|AddPlanet (Variables|Default|GetUI) _array_element))
  (for _array_element_2 (Variables|Default|GetSpacecrafts)
    (Default|AddSpacecraft (Variables|Default|GetUI) _array_element_2))
  ;[1 1 1] UI Focus request
  (EventDispatchers|BindEventtoFocusRequest (Variables|Default|GetUI) (delegate Custom|Focus)))

(event Custom|Add%20Spacecraft
  (params (Spacecraft :type Rocket%20Object%20Reference) (Planet :type Integer))
  (bind _planets (Variables|Default|GetPlanets))
  (bind _output (Utilities|Array|Get(acopy) _planets Planet))
  (bind _root (Variables|/Script/GameBehaviour.Planet|GetRoot _output))
  (bind _returnvalue (Math|Vector|GetForwardVector _root))
  ;[1 1 1] Register an existing spacecraft
  (Transformation|AttachActorToActor Spacecraft _output "None" "KeepWorld" "KeepWorld" "KeepWorld" false)
  (Transformation|SetActorRelativeTransform Spacecraft (Math|Transform|MakeTransform (+ (* _returnvalue (* 1e+02 (Variables|/Script/GameBehaviour.Planet|GetPlanetScale _output))) (* _returnvalue (* (/ (Default|GetRocketHeight Spacecraft) 2.0) 0.002))) (Class|KismetMathLibrary|MakeRotfromYZ (Transformation|GetActorUpVector) _returnvalue) "0.002000,0.002000,0.002000") false true)
  (Utilities|Array|Add (Variables|Default|GetSpacecrafts) Spacecraft)
  (Variables|/Script/GameBehaviour.OrbitalBody|SetParent Spacecraft _output)
  (Variables|/Script/GameBehaviour.Spacecraft|SetSolarSystem Spacecraft (Variables|Default|GetPlanets))
  (Variables|Default|SetLaunchpad%20Busy true))

(event Custom|On%20Rocket%20Exploded
  (params (Rocket :type Rocket%20Object%20Reference))
  ;[1 1 1] Removes rocket from UI and tracker
  (Utilities|Array|RemoveItem (Variables|Default|GetSpacecrafts) Rocket)
  (Default|RemoveSpacecraft (Variables|Default|GetUI) Rocket))

(event EventBeginPlay
  (bind _planets (Variables|Default|GetPlanets))
  (bind _output (Utilities|Array|Get(acopy) _planets))
  ;[1 1 1] Setup planets and UI
  (Pawn|Possess (Game|GetPlayerController 0) self)
  (for _array_element (Variables|Default|GetSolar%20System%20Configuration)
    (bind _returnvalue (Game|SpawnActorfromClass (.type _array_element) (Math|Transform|MakeTransform (Utilities|RandomPlanetLocation (.distance _array_element)) "0, 0, 0" "1,1,1") "AdjustIfPossibleButAlwaysSpawn" self 0))
    (Utilities|Array|Add (Variables|Default|GetPlanets) _returnvalue)
    (Variables|/Script/GameBehaviour.Planet|SetSun _returnvalue _output)
    (Transformation|AttachComponentToComponent _returnvalue (Variables|Components|GetSolar%20System) "None" "KeepRelative" "KeepRelative" "KeepRelative" false)
    (Class|Planet|Orbit _returnvalue _output))
  (CallFunction|Focus (Utilities|Array|Get(acopy) (Variables|Default|GetPlanets) (Variables|Default|GetDefault%20Focus)))
  (bind _returnvalue_2 (Actor|GetActorOfClass "/Script/Engine.DirectionalLight"))
  (Variables|Default|SetLight _returnvalue_2)
  (CallFunction|GenerateUI))

(event EventTick
  (params (DeltaSeconds :type Float%20%28single-precision%29))
  (bind _focus_craft (Variables|Default|GetFocus%20Craft))
  (bind _camera_pivot (Variables|Components|GetCamera%20Pivot))
  (bind _gimbal (Variables|Components|GetGimbal))
  (bind _focus_target (Variables|Default|GetFocus%20Target))
  (bind _relativerotation (Variables|/Script/Engine.SceneComponent|GetRelativeRotation _gimbal))
  (bind _torque (Variables|/Game/Blueprint/Actors/Rocket.Rocket_C|GetTorque _focus_craft))
  (if (not (Variables|Default|GetPaused))
    (Utilities|FlowControl|Sequence
      (:then_0
        ;[1 1 1] Focus on body/vessel
        (Utilities|IsValid _focus_target
          (:Is%20Valid
            (Transformation|SetWorldLocation (Variables|Components|GetCamera%20Pivot) (Math|Vector|Lerp(Vector) (Transformation|GetWorldLocation (Variables|Components|GetCamera%20Pivot)) (Transformation|GetActorLocation _focus_target) (stale Custom|Focus _value)) false true)
            (bind _asrocket (Utilities|Casting|CastToRocket (Variables|Default|GetFocus%20Target))
              (:then
                (switch Utilities|FlowControl|Switch|SwitchonCameraMode (Variables|Default|GetCamera%20Mode)
                  (:NewEnumerator0
                    (bind _output_get (Variables|Default|SetCamera%20Pan%20Up%20Axis (Math|Vector|Normalize (- (Transformation|GetActorLocation _asrocket) (Transformation|GetActorLocation (Variables|/Script/GameBehaviour.OrbitalBody|GetParent _asrocket)))))))
                  (:NewEnumerator1
                    (Variables|Default|SetCamera%20Pan%20Up%20Axis (Transformation|GetActorUpVector) :!label _label))))
              (:CastFailed
                (goto _label)))
            (Transformation|SetWorldRotation _camera_pivot (Math|Rotator|Lerp(Rotator) (Transformation|GetWorldRotation _camera_pivot) (Math|Rotator|MakeRotfromZ _output_get) 0.05 true) false true))))
      (:then_1
        ;[1 1 1] Panning
        (if (Variables|Default|GetPanning)
          (Transformation|SetRelativeRotation (Variables|Components|GetGimbal) (Math|Rotator|MakeRotator 0.0 (Math|Float|Clamp(Float) (+ (.pitch _relativerotation) (Input|AxisValues|GetYAxis)) -89.0 89.0) (+ (.yaw _relativerotation) (Input|AxisValues|GetXAxis))) false false)))
      (:then_2
        ;[1 1 1] Force light to face us
        (Transformation|SetActorRotation (Variables|Default|GetLight) (Math|Conversions|RotationFromXVector (Math|Vector|Normalize (Transformation|GetWorldLocation (Variables|Components|GetCamera%20Pivot)))))
        ;[1 1 1] Input system
        (Utilities|IsValid _focus_craft
          (:Is%20Valid
            (if (Variables|/Game/Blueprint/Actors/Rocket.Rocket_C|GetIs%20Deployed _focus_craft)
              (Class|Spacecraft|SetInput _focus_craft (Math|Rotator|MakeRotator (* _torque (Input|AxisValues|GetVertical)) (* _torque (Input|AxisValues|GetHorizontal)) (* _torque (Input|AxisValues|GetRoll)))))))))))

(event Input|AxisEvents|InputAxisZoom
  (params (AxisValue :type Float%20%28single-precision%29))
  ;[1 1 1] Zoom in/out
  (Utilities|IsValid (Variables|Default|GetFocus%20Target)
    (:Is%20Valid
      (bind _output_get (Variables|Default|SetZoom (Math|Float|Max(Float) (+ (* AxisValue -1.0) (Variables|Default|GetZoom)) 0.1)))
      (bind _offset (CallFunction|GetOffset (Variables|Default|GetFocus%20Target)))
      (Transformation|SetRelativeLocation (Variables|Components|GetPlayer%20Camera) (* (Math|Vector|Normalize (Variables|/Script/Engine.SceneComponent|GetRelativeLocation (Variables|Components|GetPlayer%20Camera))) (* _output_get _offset)) false true))))

(event Input|KeyboardEvents|Comma
  (params (Key :type Key%20Structure :default "None"))
  ;[1 1 1] Switch focus
  (:Pressed
    (bind _result (Math|Integer|DecrementInt (Variables|Default|GetDefault%20Focus))
      (:%20%20
        (Variables|Default|SetDefault%20Focus (Math|Integer|Clamp(Integer) _result 0 (Utilities|Array|Length (Variables|Default|GetPlanets))))
        (CallFunction|Focus (Utilities|Array|Get(acopy) (Variables|Default|GetPlanets) (Math|Integer|Clamp(Integer) _result 0 (Utilities|Array|Length (Variables|Default|GetPlanets)))))))))

(event Input|KeyboardEvents|Period
  (params (Key :type Key%20Structure :default "None"))
  ;[1 1 1] Switch focus
  (:Pressed
    (bind _result (Math|Integer|IncrementInt (Variables|Default|GetDefault%20Focus))
      (:%20%20
        (Variables|Default|SetDefault%20Focus (Math|Integer|Clamp(Integer) _result 0 (Utilities|Array|Length (Variables|Default|GetPlanets))))
        (CallFunction|Focus (Utilities|Array|Get(acopy) (Variables|Default|GetPlanets) (Math|Integer|Clamp(Integer) _result 0 (Utilities|Array|Length (Variables|Default|GetPlanets)))))))))

(event Input|KeyboardEvents|SpaceBar
  (params (Key :type Key%20Structure :default "None"))
  (bind _focus_craft (Variables|Default|GetFocus%20Craft))
  ;[1 1 1] Rocket deployment
  (:Pressed
    (if (and (Utilities|IsValid _focus_craft) (not (Variables|/Game/Blueprint/Actors/Rocket.Rocket_C|GetIs%20Deployed _focus_craft)))
      (Default|Deploy _focus_craft)
      (Transformation|AttachComponentToComponent _focus_craft (Variables|Components|GetSolar%20System) "None" "KeepWorld" "KeepWorld" "KeepWorld" true)
      (Class|OrbitalBody|AddImpulse _focus_craft (Variables|/Script/GameBehaviour.OrbitalBody|GetVelocity _focus_craft))
      (Class|OrbitalBody|AddImpulse _focus_craft (* (Transformation|GetActorUpVector _focus_craft) (Variables|Default|GetEjection%20Force)))
      (Class|Spacecraft|SetThrottleDirection _focus_craft 1.0)
      (Variables|Default|SetLaunchpad%20Busy false))))

(event Input|MouseEvents|RightMouseButton
  (params (Key :type Key%20Structure :default "None"))
  ;[1 1 1] Enable/disable panning
  (:Pressed
    (Variables|Default|SetPanning true)
    (Input|SetInputModeGameOnly (Game|GetPlayerController 0)))
  (:Released
    (Variables|Default|SetPanning false)
    (Input|SetInputModeGameandUI (Game|GetPlayerController 0) (Variables|Default|GetUI) "DoNotLock" true)))

(event Input|KeyboardEvents|LeftCtrl
  (params (Key :type Key%20Structure :default "None"))
  (bind _focus_craft (Variables|Default|GetFocus%20Craft))
  ;[1 1 1] Throttle control
  (:Pressed
    (Utilities|IsValid (Variables|Default|GetFocus%20Craft)
      (:Is%20Valid
        (Class|Spacecraft|SetThrottleDirection _focus_craft -1.0))))
  (:Released
    (Utilities|IsValid (Variables|Default|GetFocus%20Craft)
      (:Is%20Valid
        (Class|Spacecraft|SetThrottleDirection _focus_craft 0.0)))))

(event Input|KeyboardEvents|LeftShift
  (params (Key :type Key%20Structure :default "None"))
  (bind _focus_craft (Variables|Default|GetFocus%20Craft))
  ;[1 1 1] Throttle control
  (:Pressed
    (Utilities|IsValid (Variables|Default|GetFocus%20Craft)
      (:Is%20Valid
        (Class|Spacecraft|SetThrottleDirection _focus_craft 1.0))))
  (:Released
    (Utilities|IsValid (Variables|Default|GetFocus%20Craft)
      (:Is%20Valid
        (Class|Spacecraft|SetThrottleDirection _focus_craft 0.0)))))

(event Input|KeyboardEvents|X
  (params (Key :type Key%20Structure :default "None"))
  (bind _focus_craft (Variables|Default|GetFocus%20Craft))
  ;[1 1 1] Throttle control
  (:Pressed
    (Utilities|IsValid _focus_craft
      (:Is%20Valid
        (Class|Spacecraft|SetThrottleDirection _focus_craft 0.0)
        (Variables|/Game/Blueprint/Actors/Rocket.Rocket_C|SetThrottle _focus_craft 0.0)))))

(event Input|KeyboardEvents|Z
  (params (Key :type Key%20Structure :default "None"))
  (bind _focus_craft (Variables|Default|GetFocus%20Craft))
  ;[1 1 1] Throttle control
  (:Pressed
    (Utilities|IsValid _focus_craft
      (:Is%20Valid
        (Class|Spacecraft|SetThrottleDirection _focus_craft 0.0)
        (Variables|/Game/Blueprint/Actors/Rocket.Rocket_C|SetThrottle _focus_craft 1.0)))))

(event Input|KeyboardEvents|C
  (params (Key :type Key%20Structure :default "None"))
  ;[1 1 1] Switch camera mode
  (:Pressed
    (Utilities|IsValid (Variables|Default|GetFocus%20Craft)
      (:Is%20Valid
        (switch Utilities|FlowControl|Switch|SwitchonCameraMode (Variables|Default|GetCamera%20Mode)
          (:NewEnumerator0
            (Variables|Default|SetCamera%20Mode "NewEnumerator1"))
          (:NewEnumerator1
            (Variables|Default|SetCamera%20Mode "NewEnumerator0")))))))

(fn ConstructionScript)

(fn GetOffset
  (params (Target :type Actor%20Object%20Reference))
  (bind _asplanet (Utilities|Casting|CastToPlanet Target)
    (:then
      (return (Class|Planet|GetUnitsRadius _asplanet)))
    (:CastFailed
      (return 0.8))))

(fn SetPaused
  (params (Paused :type Boolean))
  (bind _output_get (Variables|Default|SetPaused Paused))
  (for _array_element (Variables|Default|GetPlanets)
    (Rendering|SetVisibility (Variables|/Script/GameBehaviour.Planet|GetRoot _array_element) (not _output_get) true))
  (for _array_element_2 (Variables|Default|GetSpacecrafts)
    (Rendering|SetVisibility (Variables|/Script/Engine.Actor|GetRootComponent _array_element_2) (not _output_get) true)
    (Default|OnVisibilityChanged _array_element_2 (not _output_get)))
  (if (not _output_get)
    (Pawn|Possess (Game|GetPlayerController 0) self)
    (CallFunction|GenerateUI)))

(fn SpawnActorinSystem
  (params (Type :type Actor%20Class%20Reference) (Location :type Vector) (Rotation :type Rotator) (Scale :type Vector :default "1.000000,1.000000,1.000000") (Attach%20To :type Actor%20Object%20Reference))
  (bind _returnvalue (Game|SpawnActorfromClass Type (Math|Transform|MakeTransform Location Rotation Scale) "Undefined" 0 0))
  (if (Utilities|IsValid Attach%20To)
    (Transformation|AttachActorToActor _returnvalue Attach%20To "None" "KeepWorld" "KeepWorld" "KeepWorld" false)
    (else
      (Transformation|AttachComponentToComponent _returnvalue (Variables|Components|GetSolar%20System) "None" "KeepWorld" "KeepWorld" "KeepWorld" false)))
  (return _returnvalue))