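; EditorController is the possessed actor that runs the rocket editor, letting the player assemble a single-stage rocket from parts.
; It spawns a half-scale Rocket and binds RocketEditor widget buttons to add fuel or engine, remove, and clear.
; An engine closes the stage, blocking further additions until removal or clearing.
; Part edits refresh fuel and mass readouts and shift a focus height, toward which Tick lerps the rocket.
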(event Custom|On%20Root%20Added
  ;[1 1 1] Add Command Pod
  (Default|ShowError (Variables|Default|GetUI) "Cannot attach a second command pod to this stage." 2.5))

(event Custom|On%20Fuel%20Added
  ;[1 1 1] Add Fuel Tank
  (CallFunction|AddPartbyType "/Game/Blueprint/Components/Rocket_FuelModule.Rocket_FuelModule_C"))

(event Custom|Refresh%20Mass
  (Default|UpdateTotalMass (Variables|Default|GetUI) (/ (Default|CalculateMass (Variables|Default|GetBuilder)) 1e+03)))

(event Custom|On%20Engine%20Added
  ;[1 1 1] Add Engine
  (CallFunction|AddPartbyType "/Game/Blueprint/Components/Rocket_EngineModule.Rocket_EngineModule_C")
  (Variables|Default|SetStage%20Building false))

(event Custom|Add%20Part%20By%20Type
  (params (Type :type Rocket%20Part%20Class%20Reference))
  (if (Variables|Default|GetStage%20Building)
    (Default|AddPart (Variables|Default|GetBuilder) Type)
    (Variables|Default|SetFocus%20Height (+ (Variables|Default|GetFocus%20Height) 146.5))
    (Default|UpdateTotalFuel (Variables|Default|GetUI) (Default|GetTotalFuel (Variables|Default|GetBuilder)))
    (CallFunction|RefreshMass)
    (else
      (Default|ShowError (Variables|Default|GetUI) "Separate stages are not supported at this time." 2.5))))

(event Custom|On%20Part%20Removed
  ;[1 1 1] Remove Last Part
  (Variables|Default|SetStage%20Building true)
  (bind _removed (Default|RemoveLastPart (Variables|Default|GetBuilder)))
  (if _removed
    (Variables|Default|SetFocus%20Height (- (Variables|Default|GetFocus%20Height) 146.0))
    (Default|UpdateTotalFuel (Variables|Default|GetUI) (Default|GetTotalFuel (Variables|Default|GetBuilder)))
    (CallFunction|RefreshMass)))

(event Custom|On%20Parts%20Cleared
  ;[1 1 1] Remove All Parts
  (Default|RemoveAllParts (Variables|Default|GetBuilder))
  (Variables|Default|SetFocus%20Height 0.0)
  (Variables|Default|SetStage%20Building true)
  (Default|UpdateTotalFuel (Variables|Default|GetUI) (Default|GetTotalFuel (Variables|Default|GetBuilder)))
  (CallFunction|RefreshMass))

(event EventBeginPlay
  (Pawn|Possess (Game|GetPlayerController 0) self)
  (bind _returnvalue (Game|SpawnActorfromClass "/Game/Blueprint/Actors/Rocket.Rocket_C" (Math|Transform|MakeTransform "0, 0, 0" "0, 0, 0" "0.500000,0.500000,0.500000") "AlwaysSpawn" 0 0))
  (Variables|Default|SetBuilder _returnvalue)
  (bind _foundwidgets (Widget|GetAllWidgetsOfClass "/Game/Blueprint/UI/RocketEditor.RocketEditor_C" true))
  (Variables|Default|SetUI (Utilities|Array|Get(acopy) _foundwidgets))
  (CallFunction|RefreshMass)
  (Utilities|FlowControl|Sequence
    (:then_0
      (EventDispatchers|BindEventtoOnClicked (Variables|/Game/Blueprint/UI/RocketEditor.RocketEditor_C|GetRoot (Variables|Default|GetUI)) (delegate Custom|On%20Root%20Added)))
    (:then_1
      (EventDispatchers|BindEventtoOnClicked (Variables|/Game/Blueprint/UI/RocketEditor.RocketEditor_C|GetFuel (Variables|Default|GetUI)) (delegate Custom|On%20Fuel%20Added)))
    (:then_2
      (EventDispatchers|BindEventtoOnClicked (Variables|/Game/Blueprint/UI/RocketEditor.RocketEditor_C|GetThruster (Variables|Default|GetUI)) (delegate Custom|On%20Engine%20Added)))
    (:then_3
      (EventDispatchers|BindEventtoOnClicked (Variables|/Game/Blueprint/UI/RocketEditor.RocketEditor_C|GetRemove (Variables|Default|GetUI)) (delegate Custom|On%20Part%20Removed)))
    (:then_4
      (EventDispatchers|BindEventtoOnClicked (Variables|/Game/Blueprint/UI/RocketEditor.RocketEditor_C|GetClear (Variables|Default|GetUI)) (delegate Custom|On%20Parts%20Cleared)))))

(event EventTick
  (params (DeltaSeconds :type Float%20%28single-precision%29))
  (bind _builder (Variables|Default|GetBuilder))
  (bind _returnvalue (Transformation|GetActorLocation _builder))
  (Transformation|SetActorLocation (Variables|Default|GetBuilder) (Math|Vector|MakeVector (.x _returnvalue) (.y _returnvalue) (Math|Float|Lerp (.z _returnvalue) (Variables|Default|GetFocus%20Height) 0.25)) false true))

(fn ConstructionScript)