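; Agent actor that launches spacecraft on its own from an associated planet.
; Each Think event rolls a random float and, if it exceeds ChanceOfSpawning while the launchpad is free, asks SolarSystem to spawn one of three random rocket types without adding it to the UI.
; A higher ChanceOfSpawning therefore means fewer launches.
; Spawning marks the launchpad busy, and this graph never clears that flag.
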(event Custom|Think
  (if (and (> (Math|Random|RandomFloat) (Variables|Default|GetChance%20of%20Spawning)) (not (Variables|Default|GetLaunchpad%20Busy)))
    (Default|SpawnSpacecraft (Variables|Default|GetSolar%20System) (Variables|Default|GetPlanet) (Utilities|Array|Get(acopy) (Variables|Default|GetRocket%20Types) (Math|Random|RandomIntegerinRange 0 2)) false)
    (Variables|Default|SetLaunchpad%20Busy true)))