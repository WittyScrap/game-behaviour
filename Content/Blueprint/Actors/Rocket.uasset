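; Modular player-controlled rocket actor that is built from stacked part components, deployed into physics, and explodes on hitting a planet.
; Parts attach downward under the current stage, refreshing Core's modules and resizing the capsule to the stack height.
; Throttle ramps each tick into Core, which also takes roll, pitch and yaw, while summed part mass overrides the capsule's mass.
; Deploy starts physics and destroys the engine clamps; focus events toggle marker visibility.
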(event Custom|Add%20Part
  (params (Part%20Type :type Rocket%20Part%20Class%20Reference))
  ;[1 1 1] Adds a new part to this rocket of a specific type to the bottom
  (bind _returnvalue (Class|ActorUtilities|AddComponentbyClass self Part%20Type))
  (bind _asrocket_part (Utilities|Casting|CastToRocketPart _returnvalue))
  (Transformation|SetRelativeLocation _asrocket_part (Math|Vector|MakeVector 0.0 0.0 (- (.z (Variables|/Script/Engine.SceneComponent|GetRelativeLocation (Utilities|Array|Get(acopy) (Variables|Default|GetParts) (- (Utilities|Array|Length (Variables|Default|GetParts)) 1)))) 293.0)) false true)
  (Collision|SetCollisionEnabled _asrocket_part "NoCollision")
  (Physics|SetSimulatePhysics _asrocket_part false)
  (Utilities|Array|Add (Variables|Default|GetParts) _asrocket_part)
  (Transformation|AttachComponentToComponent _asrocket_part (Variables|Default|GetCurrent%20Stage) "None" "KeepRelative" "KeepRelative" "KeepRelative" true)
  (Default|RefreshModules (Variables|Default|GetCore))
  (CallFunction|UpdateCollision))

(event Custom|Update%20Collision
  ;[1 1 1] Update the capsule collision
  (Components|Capsule|SetCapsuleRadius (Variables|Default|GetCollision) 1e+02 false)
  (Components|Capsule|SetCapsuleHalfHeight (Variables|Default|GetCollision) (/ (CallFunction|GetRocketHeight) 2.0) false))

(event Custom|Deploy
  ;[1 1 1] Start physics
  (Physics|SetSimulatePhysics (Variables|Default|GetCollision) true)
  (Variables|Default|SetIs%20Deployed true)
  (bind _asrocket_engine_module (Utilities|Casting|CastToRocket_EngineModule (Utilities|Array|Get(acopy) (Variables|Default|GetParts) (Utilities|Array|LastIndex (Variables|Default|GetParts)))))
  (bind _returnvalue (Game|SpawnActorfromClass "/Game/Blueprint/Actors/Explosion.Explosion_C" (Transformation|GetWorldTransform (Variables|/Game/Blueprint/Components/Rocket_EngineModule.Rocket_EngineModule_C|GetClamps _asrocket_engine_module)) "Undefined" 0 0))
  (Transformation|AttachActorToActor _returnvalue (Variables|Default|GetParent) "None" "KeepWorld" "KeepWorld" "KeepWorld" true)
  (Components|DestroyComponent (Variables|/Game/Blueprint/Components/Rocket_EngineModule.Rocket_EngineModule_C|GetClamps _asrocket_engine_module))
  (CallFunction|OnFocus))

(event Custom|Remove%20All%20Parts
  ;[1 1 1] Clears all parts from the rocket
  (bind _removed (CallFunction|RemoveLastPart :!label _label))
  (if _removed
    (goto _label)))

(event Custom|Recenter
  ;[1 1 1] Updates the center of mass for the rocket
  (Transformation|AddLocalOffset (Variables|Default|GetStage0) (Math|Vector|MakeVector 0.0 0.0 (/ (- (CallFunction|GetRocketHeight) (Variables|Default|GetPart%20Height)) 2.0)) false true))

(event Custom|On%20Focus
  ;[1 1 1] Focus control - enables or disables markers visibility
  (if (Variables|Default|GetIs%20Deployed)
    (CallFunction|ToggleUI true)))

(event Custom|On%20Focus%20Lost
  ;[1 1 1] Focus control - enables or disables markers visibility
  (if (Variables|Default|GetIs%20Deployed)
    (CallFunction|ToggleUI false)))

(event Custom|On%20Visibility%20Changed
  (params (Visibility :type Boolean))
  ;[1 1 1] Focus control - enables or disables markers visibility
  (if Visibility
    (if (Variables|Default|GetUI%20Shown)
      (CallFunction|OnFocus)
      (else
        (CallFunction|ToggleUI false)))))

(event Custom|Toggle%20UI
  (params (Visible :type Boolean))
  (Rendering|SetVisibility (Variables|Default|GetMarkers) Visible true)
  (Variables|Default|SetUI%20Shown true))

(event EventOnThrottleDirectionSet
  (params (throttling :type Float%20%28single-precision%29))
  ;[1 1 1] Sets the "direction" for the throttle, AKA whether we are throttling UP or DOWN.
  (Variables|Default|SetThrottle%20Direction throttling))

(event EventOnInputSet
  (params (throttling :type Rotator :default "0, 0, 0"))
  ;[1 1 1] Roll, Pitch, and Yaw control
  (Default|Roll (Variables|Default|GetCore) (.roll throttling))
  (Default|Pitch (Variables|Default|GetCore) (.pitch throttling))
  (Default|Yaw (Variables|Default|GetCore) (.yaw throttling)))

(event EventBeginPlay
  ;[1 1 1] Begin Play
  (Utilities|Array|Add (Variables|Default|GetParts) (Variables|Default|GetCore))
  (Variables|Default|SetCurrent%20Stage (Variables|Default|GetStage0))
  (CallFunction|UpdateCollision))

(event EventTick
  (params (DeltaSeconds :type Float%20%28single-precision%29))
  ;[1 1 1] Set throttle and update craft mass
  (bind _output_get (Variables|Default|SetThrottle (Math|Float|Clamp(Float) (+ (Variables|Default|GetThrottle) (* DeltaSeconds (Variables|Default|GetThrottle%20Sensitivity) (Variables|Default|GetThrottle%20Direction))))))
  (Default|Throttle (Variables|Default|GetCore) _output_get)
  (CallFunction|UpdateMass))

(event Collision|EventHit
  (params (MyComp :type Primitive%20Component%20Object%20Reference) (Other :type Actor%20Object%20Reference) (OtherComp :type Primitive%20Component%20Object%20Reference) (bSelfMoved :type Boolean) (HitLocation :type Vector :default "0, 0, 0") (HitNormal :type Vector :default "0, 0, 0") (NormalImpulse :type Vector :default "0, 0, 0") (Hit :type Hit%20Result%20Structure%20%28by%20ref%29))
  ;[1 1 1] Attack and destroy
  (bind _asplanet (Utilities|Casting|CastToPlanet Other))
  (bind _returnvalue (Actor|GetActorOfClass "/Game/Blueprint/Actors/PlayerSystem.PlayerSystem_C"))
  (Default|Focus _returnvalue _asplanet)
  (Default|SpawnActorinSystem _returnvalue "/Game/Blueprint/Actors/Explosion.Explosion_C" (Transformation|GetActorLocation) (Transformation|GetActorRotation) "0.010000,0.010000,0.010000")
  (Default|OnRocketExploded _returnvalue self)
  (Actor|DestroyActor))

(fn ConstructionScript
  (Collision|SetCollisionEnabled (Variables|Default|GetCollision) "PhysicsOnly")
  (Collision|SetCollisionEnabled (Variables|Default|GetCore) "PhysicsOnly"))

(fn RemoveLastPart
  (bind _parts (Variables|Default|GetParts))
  (bind _parts_2 (Variables|Default|GetParts))
  (bind _returnvalue (Utilities|Array|Length _parts_2))
  (bind _returnvalue_2 (- _returnvalue 1))
  (bind _output (Utilities|Array|Get(acopy) _parts _returnvalue_2))
  (if (> _returnvalue 1)
    (Utilities|FlowControl|Sequence
      (:then_0
        (bind _asrocket_engine_module (Utilities|Casting|CastToRocket_EngineModule _output))
        (Components|DestroyComponent (Variables|/Game/Blueprint/Components/Rocket_EngineModule.Rocket_EngineModule_C|GetThruster%20Effect _asrocket_engine_module))
        (Components|DestroyComponent (Variables|/Game/Blueprint/Components/Rocket_EngineModule.Rocket_EngineModule_C|GetClamps _asrocket_engine_module)))
      (:then_1
        (Components|DestroyComponent _output)
        (Utilities|Array|RemoveIndex (Variables|Default|GetParts) (- (Utilities|Array|Length (Variables|Default|GetParts)) 1))
        (Default|RefreshModules (Variables|Default|GetCore))
        (return true)))
    (else
      (return false))))

(fn GetTotalFuel
  (for _array_element (Variables|Default|GetParts)
    (bind _asrocket_fuel_module (Utilities|Casting|CastToRocket_FuelModule _array_element))
    (LocalVariables|SetTotal (+ (Default|GetFuel _asrocket_fuel_module) (LocalVariables|GetTotal))))
  (return (LocalVariables|GetTotal)))

(fn UpdateMass
  (bind _output_get (Variables|Default|SetMass (CallFunction|CalculateMass)))
  (Class|PrimitiveComponent|SetMassOverrideinKg (Variables|Default|GetCollision) "None" _output_get true))

(fn CalculateMass
  (for _array_element (Variables|Default|GetParts)
    (LocalVariables|SetTotal%20Mass (+ (Default|GetMass _array_element) (LocalVariables|GetTotal%20Mass))))
  (return (LocalVariables|GetTotal%20Mass)))

(fn AddMesh
  (params (Mesh :type Static%20Mesh%20Object%20Reference) (Material :type Material%20Object%20Reference) (Location :type Vector) (Rotation :type Rotator) (Attach%20To :type Scene%20Component%20Object%20Reference))
  (bind _returnvalue (Class|ActorUtilities|AddComponentbyClass self "/Script/Engine.StaticMeshComponent"))
  (bind _asstatic_mesh_component (Utilities|Casting|CastToStaticMeshComponent _returnvalue))
  (Components|StaticMesh|SetStaticMesh _asstatic_mesh_component Mesh)
  (Rendering|Material|SetMaterial _asstatic_mesh_component 0 Material)
  (Transformation|SetRelativeLocationAndRotation _asstatic_mesh_component Location Rotation false true)
  (Transformation|AttachComponentToComponent _asstatic_mesh_component Attach%20To "None" "KeepRelative" "KeepRelative" "KeepRelative" true)
  (return _asstatic_mesh_component))

(fn GetRocketHeight
  (return (* (Utilities|Array|Length (Variables|Default|GetParts)) (Variables|Default|GetPart%20Height))))

(fn AddMeshMultipleMaterials
  (params (Mesh :type Static%20Mesh%20Object%20Reference) (Materials :type Array%20of%20Material%20Object%20References) (Location :type Vector) (Rotation :type Rotator) (Attach%20To :type Scene%20Component%20Object%20Reference))
  (bind _returnvalue (Class|ActorUtilities|AddComponentbyClass self "/Script/Engine.StaticMeshComponent"))
  (bind _asstatic_mesh_component (Utilities|Casting|CastToStaticMeshComponent _returnvalue))
  (Components|StaticMesh|SetStaticMesh _asstatic_mesh_component Mesh)
  (for (_array_element _array_index) Materials
    (Rendering|Material|SetMaterial _asstatic_mesh_component _array_index _array_element))
  (Transformation|SetRelativeLocationAndRotation _asstatic_mesh_component Location Rotation false true)
  (Transformation|AttachComponentToComponent _asstatic_mesh_component Attach%20To "None" "KeepRelative" "KeepRelative" "KeepRelative" true)
  (return _asstatic_mesh_component))